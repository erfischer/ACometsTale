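; BlueStarPower is a collectible pickup that adds a fixed amount of StarPower to the CometCharacter.
; When a movable comet overlaps the CollisionSphere, it grants the power, hides the Sphere, and plays a burst particle and 2D sound.
; The actor destroys itself after a short delay, leaving collision active meanwhile, so a repeat overlap can grant power again.
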(event OnComponentBeginOverlap(CollisionSphere)
  (params (OverlappedComponent :type Primitive%20Component%20Object%20Reference) (OtherActor :type Actor%20Object%20Reference) (OtherComp :type Primitive%20Component%20Object%20Reference) (OtherBodyIndex :type Integer) (bFromSweep :type Boolean) (SweepResult :type Hit%20Result%20Structure%20%28by%20ref%29))
  (bind _ascomet_character (Utilities|Casting|CastToCometCharacter OtherActor))
  (if (Variables|/Game/CometsTaleBP/Blueprints/CometCharacter.CometCharacter_C|GetCanMove _ascomet_character)
    (Variables|/Game/CometsTaleBP/Blueprints/CometCharacter.CometCharacter_C|SetStarPower _ascomet_character (+ (Variables|/Game/CometsTaleBP/Blueprints/CometCharacter.CometCharacter_C|GetStarPower _ascomet_character) 300))
    (Rendering|SetVisibility (Variables|Default|GetSphere) false false)
    (Effects|SpawnEmitteratLocation "/Game/CometsTaleBP/Blueprints/ParticleEffects/BlueCollectBurst.BlueCollectBurst" (Transformation|GetActorLocation))
    (Audio|PlaySound2D "/Game/CometsTaleBP/Blueprints/Sounds/171646__fins__scale-e6.171646__fins__scale-e6")
    (Utilities|FlowControl|Delay 1.3)
    (Actor|DestroyActor)))

(event EventBeginPlay)

(event Collision|EventActorBeginOverlap
  (params (OtherActor :type Actor%20Object%20Reference)))

(event EventTick
  (params (DeltaSeconds :type Float%20%28single-precision%29)))

(fn ConstructionScript)