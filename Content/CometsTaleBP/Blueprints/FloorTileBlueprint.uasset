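; Endless-runner floor tile that extends the track as the comet character passes through it.
; When CometCharacter overlaps EndTrigger, it has FlygameMode add a floor tile, then destroys itself after a short delay.
; GetAttachTransform exposes the AttachPoint world transform.
; The construction script spawns StarPower actors at random points in SpawnArea's box, using its relative location as the origin.
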(event OnComponentBeginOverlap(EndTrigger)
  (params (OverlappedComponent :type Primitive%20Component%20Object%20Reference) (OtherActor :type Actor%20Object%20Reference) (OtherComp :type Primitive%20Component%20Object%20Reference) (OtherBodyIndex :type Integer) (bFromSweep :type Boolean) (SweepResult :type Hit%20Result%20Structure%20%28by%20ref%29))
  (Utilities|Casting|CastToCometCharacter OtherActor)
  (bind _asflygame_mode (Utilities|Casting|CastToFlygameMode (Game|GetGameMode)))
  (Default|AddFloorTile _asflygame_mode)
  (Utilities|FlowControl|Delay 2.0)
  (Actor|DestroyActor))

(event EventBeginPlay)

(event Collision|EventActorBeginOverlap
  (params (OtherActor :type Actor%20Object%20Reference)))

(event EventTick
  (params (DeltaSeconds :type Float%20%28single-precision%29)))

(fn ConstructionScript
  (CallFunction|SpawnStarPower))

(fn GetAttachTransform
  (return (Transformation|GetWorldTransform (Variables|Default|GetAttachPoint))))

(fn SpawnStarPower
  (bind _spawnarea (Variables|Default|GetSpawnArea))
  (for _index (range 0 10)
    (Game|SpawnActorfromClass "/Game/CometsTaleBP/Blueprints/StarPower.StarPower_C" (Math|Conversions|ToTransform(Vector) (Math|Random|RandomPointinBoundingBox (Variables|/Script/Engine.SceneComponent|GetRelativeLocation _spawnarea) (Variables|/Script/Engine.BoxComponent|GetBoxExtent _spawnarea))) "Undefined" 0 0)))